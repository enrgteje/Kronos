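; BP_Spawner is a spawner actor that places an enemy in the level when play begins.
; BeginPlay calls a SpawnEnemy custom event, which spawns the class held in the Enemy variable at the SpawnPoint component's world transform.
; A delayed spawn using SpawnDelay exists but is not connected, so the actor itself triggers only that single spawn.
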(event Custom|Spawn%20Enemy
  (params (Enemy :type Actor%20Class%20Reference) (SpawnTransform :type Transform))
  (Game|SpawnActorfromClass Enemy SpawnTransform "Undefined" 0 0))

(event EventBeginPlay
  (CallFunction|SpawnEnemy (Variables|Default|GetEnemy) (Transformation|GetWorldTransform (Variables|Default|GetSpawnPoint))))

(fn ConstructionScript)