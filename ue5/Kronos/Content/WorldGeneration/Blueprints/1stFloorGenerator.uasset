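; First-floor dungeon generator Blueprint that procedurally builds a level from room data, starting generation three seconds after BeginPlay.
; Overrides begin at a spawn room, add random rooms, and pick the end room once a minimum count is reached if none exists.
; Growth continues up to a maximum count, and validity requires an end room.
; Saloon doors join rooms, walls fill other openings, and the player moves to the generator afterward.
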(event EventBeginPlay
  (Utilities|FlowControl|Delay 3.0)
  (PCG|Generate))

(event EventOnGenerationInitBP)

(event EventOnPostGenerationBP
  (Transformation|SetActorTransform (Game|GetPlayerCharacter 0) (Math|Transform|MakeTransform (Transformation|GetActorLocation) "0, 0, 0" "1.000000,1.000000,1.000000")))

(fn ConstructionScript)

(fn ChooseFirstRoomData
  (return (Variables|Default|GetSpawn%20Room)))

(fn ChooseNextRoomData
  (params (CurrentRoom :type Room%20Data%20Object%20Reference))
  (if (and (>= (Class|DungeonGenerator|GetNbRoom) (Variables|Default|GetMinNumOfRooms)) (not (Class|DungeonGenerator|HasAlreadyRoomData (Variables|Default|GetEndRoom))))
    (return (Variables|Default|GetEndRoom))
    (else
      (bind _returnvalue (Class|DungeonGenerator|GetRandomRoomData (Variables|Default|GetRooms)))
      (return _returnvalue))))

(fn ContinuetoAddRoom
  (return (<= (Class|DungeonGenerator|GetNbRoom) (Variables|Default|GetMaxNumOfRooms))))

(fn IsValidDungeon
  (return (Class|DungeonGenerator|HasAlreadyRoomData (Variables|Default|GetEndRoom))))

(fn ChooseDoor
  (params (CurrentRoom :type Room%20Data%20Object%20Reference) (NextRoom :type Room%20Data%20Object%20Reference))
  (if (and (Utilities|IsValid CurrentRoom) (Utilities|IsValid NextRoom))
    (return "/Game/WorldGeneration/Blueprints/BP_SaloonDoor.BP_SaloonDoor_C")
    (else
      (return "/Game/WorldGeneration/Blueprints/Wall.Wall_C"))))