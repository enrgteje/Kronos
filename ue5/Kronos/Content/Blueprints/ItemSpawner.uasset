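; ItemSpawner is an actor that spawns a random item and labels it with that item's name and info.
; On BeginPlay it picks a random class from ItemList and spawns it at the SpawnPoint transform.
; It then queries the spawned actor through ItemInterface to fill the ItemName and SpawnerText displays, leaving them unchanged if the interface cast fails.
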(event EventBeginPlay
  (bind _returnvalue (Game|SpawnActorfromClass (.OutItem (Utilities|Array|Random (Variables|Default|GetItemList))) (Transformation|GetWorldTransform (Variables|Default|GetSpawnPoint)) "Undefined" 0 0))
  (bind _asitem_interface (Utilities|Casting|CastToItemInterface _returnvalue))
  (bind _info (Default|GetItemInfo _asitem_interface))
  (Rendering|Components|TextRender|SetText (Variables|Default|GetSpawnerText) (Utilities|Text|ToText(String) _info))
  (bind _name (Default|GetItemName _asitem_interface))
  (Rendering|Components|TextRender|SetText (Variables|Default|GetItemName) (Utilities|Text|ToText(String) _name)))

(event Collision|EventActorBeginOverlap
  (params (OtherActor :type Actor%20Object%20Reference)))

(event EventTick
  (params (DeltaSeconds :type Float%20%28single-precision%29)))

(fn ConstructionScript)